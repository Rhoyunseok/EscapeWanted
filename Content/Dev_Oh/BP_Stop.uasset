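; BP_Stop is a trigger actor that plays the 2D voice clip "거기아니라고" ("I said not there") when its Box is overlapped.
; Any overlapping actor triggers it, at the pitch set by the Pitch variable, with no filter or one-shot guard.
; When Last is true, four more copies play simultaneously, three starting at different offsets into the clip, layering the sound.
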(event `self.Box.OnComponentBeginOverlap`
  (params (OverlappedComponent :type "PrimitiveComponent Object Reference") (OtherActor :type "Actor Object Reference") (OtherComp :type "PrimitiveComponent Object Reference") (OtherBodyIndex :type Integer) (bFromSweep :type Boolean) (SweepResult :type "HitResult Structure (by ref)"))
  (`GameplayStatics.PlaySound2D` "/Game/Dev_Oh/SFX/거기아니라고.거기아니라고" 1.0 (`self.pitch`) 0.0 null null)
  (if (`self.bLast`)
    (`GameplayStatics.PlaySound2D` "/Game/Dev_Oh/SFX/거기아니라고.거기아니라고" 1.0 (`self.pitch`) 0.0 null null)
    (`GameplayStatics.PlaySound2D` "/Game/Dev_Oh/SFX/거기아니라고.거기아니라고" 1.0 (`self.pitch`) 1.0 null null)
    (`GameplayStatics.PlaySound2D` "/Game/Dev_Oh/SFX/거기아니라고.거기아니라고" 1.0 (`self.pitch`) 1.5 null null)
    (`GameplayStatics.PlaySound2D` "/Game/Dev_Oh/SFX/거기아니라고.거기아니라고" 1.0 (`self.pitch`) 2.0 null null)))

(fn `UserConstructionScript`)