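; BP_GG is a horror-game actor with a mesh and a kill zone box that forces the player to face it on contact.
; When the horror character enters the box, its input is disabled and the controller's rotation snaps toward a point just above the mesh's head socket, computed from the camera location.
; Input returns after a short delay, with no damage or death applied here.
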(event `self.ReceiveBeginPlay`)

(event `self.KillZone_Box.OnComponentBeginOverlap`
  (params (OverlappedComponent :type "PrimitiveComponent Object Reference") (OtherActor :type "Actor Object Reference") (OtherComp :type "PrimitiveComponent Object Reference") (OtherBodyIndex :type Integer) (bFromSweep :type Boolean) (SweepResult :type "HitResult Structure (by ref)"))
  (bind _asbp_horror_player_controller (cast `/Game/Variant_Horror/Blueprints/BP_HorrorPlayerController` (`GameplayStatics.GetPlayerController` 0)))
  (bind _asbp_horror_character (cast `/Game/Variant_Horror/Blueprints/BP_HorrorCharacter` OtherActor))
  (`self.DisableInput` _asbp_horror_character _asbp_horror_player_controller)
  (`Controller.SetControlRotation` _asbp_horror_player_controller (`KismetMathLibrary.FindLookAtRotation` (`PlayerCameraManager.GetCameraLocation` (`GameplayStatics.GetPlayerCameraManager` 0)) (+ (`SceneComponent.GetSocketLocation` (`self.Mesh`) "headSocket") (0.0 0.0 33.0))))
  (`KismetSystemLibrary.Delay` 2.0)
  (`self.EnableInput` _asbp_horror_character _asbp_horror_player_controller))

(fn `UserConstructionScript`)